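; Learning Agents interactor that lets trained agents fly BP_BestPlane.
; Observations feed each plane's position, forward direction, velocity and distances to floor and ceiling.
; Four float actions drive the plane: positive throttle values set ThrottleAmount, while yaw, pitch and roll add torque to Driver around its local axes.
; Torques scale with Aircontrol through a fixed-alpha lerp from zero, and negative throttle output is ignored, so there is no braking.
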(event EventSetupObservations
  (Utilities|FlowControl|Sequence
    (:then_0
      (bind _returnvalue (Class|PositionObservation|AddPositionObservation 0 "PlanePositionObservation" 1e+02))
      (Variables|Default|SetPlanePositionObservation _returnvalue)
      (bind _returnvalue_2 (Class|DirectionObservation|AddDirectionObservation 0 "TrackDirectionObservation" 1.0))
      (Variables|Default|SetPlaneDirectionObservation _returnvalue_2))
    (:then_1
      (bind _returnvalue_3 (Class|VelocityObservation|AddVelocityObservation 0 "PlaneGlobalVelocityObservation" 2e+02))
      (Variables|Default|SetPlaneVelocityObservation _returnvalue_3))
    (:then_2
      (bind _returnvalue_4 (Class|FloatObservation|AddFloatObservation 0 "DistanceToGround" 1.0))
      (Variables|Default|SetDistanceToGround _returnvalue_4)
      (bind _returnvalue_5 (Class|FloatObservation|AddFloatObservation 0 "DistanceToCeiling" 1.0))
      (Variables|Default|SetDistance%20To%20Ceiling _returnvalue_5))))

(event EventSetObservations
  (params (AgentIds :type Array%20of%20Integers))
  (for _array_element AgentIds
    (Utilities|FlowControl|Sequence
      (:then_0
        (Class|PositionObservation|SetPositionObservation (Variables|Default|GetPlanePositionObservation) _array_element "0, 0, 0" (Transformation|GetActorLocation (Class|LearningAgentsManagerComponent|GetAgent _array_element "/Game/FlyingGame/Blueprints/BP_BestPlane.BP_BestPlane_C")) (Transformation|GetActorRotation (Class|LearningAgentsManagerComponent|GetAgent _array_element "/Game/FlyingGame/Blueprints/BP_BestPlane.BP_BestPlane_C"))))
      (:then_1
        (Class|DirectionObservation|SetDirectionObservation (Variables|Default|GetPlaneDirectionObservation) _array_element (Math|Vector|GetForwardVector (Variables|/Script/Engine.Actor|GetRootComponent (Class|LearningAgentsManagerComponent|GetAgent _array_element "/Game/FlyingGame/Blueprints/BP_BestPlane.BP_BestPlane_C"))) (Transformation|GetActorRotation (Class|LearningAgentsManagerComponent|GetAgent _array_element "/Game/FlyingGame/Blueprints/BP_BestPlane.BP_BestPlane_C"))))
      (:then_2
        (Class|VelocityObservation|SetVelocityObservation (Variables|Default|GetPlaneVelocityObservation) _array_element (Transformation|GetVelocity (Class|LearningAgentsManagerComponent|GetAgent _array_element "/Game/FlyingGame/Blueprints/BP_BestPlane.BP_BestPlane_C")) (Transformation|GetActorRotation (Class|LearningAgentsManagerComponent|GetAgent _array_element "/Game/FlyingGame/Blueprints/BP_BestPlane.BP_BestPlane_C"))))
      (:then_3
        (Class|FloatObservation|SetFloatObservation (Variables|Default|GetDistanceToGround) _array_element (Variables|/Game/FlyingGame/Blueprints/BP_BestPlane.BP_BestPlane_C|GetDistance%20To%20Floor (Class|LearningAgentsManagerComponent|GetAgent _array_element "/Game/FlyingGame/Blueprints/BP_BestPlane.BP_BestPlane_C"))))
      (:then_4
        (Class|FloatObservation|SetFloatObservation (Variables|Default|GetDistance%20To%20Ceiling) _array_element (Variables|/Game/FlyingGame/Blueprints/BP_BestPlane.BP_BestPlane_C|GetDistance%20To%20Ceiling (Class|LearningAgentsManagerComponent|GetAgent _array_element "/Game/FlyingGame/Blueprints/BP_BestPlane.BP_BestPlane_C")))))))

(event EventSetupActions
  (Utilities|FlowControl|Sequence
    (:then_0
      (bind _returnvalue (Class|FloatAction|AddFloatAction 0 "ThrottleBrakeAction" 1.0))
      (Variables|Default|SetThrottleBrakeAction _returnvalue))
    (:then_1
      (bind _returnvalue_2 (Class|FloatAction|AddFloatAction 0 "LeftRightMovement" 1.0))
      (Variables|Default|SetLeft%20Right%20Movement _returnvalue_2))
    (:then_2
      (bind _returnvalue_3 (Class|FloatAction|AddFloatAction 0 "UpDownMovement" 1.0))
      (Variables|Default|SetUp%20Down%20Movement _returnvalue_3))
    (:then_3
      (bind _returnvalue_4 (Class|FloatAction|AddFloatAction 0 "None" 1.0))
      (Variables|Default|SetRoll%20Movement _returnvalue_4))))

(event EventGetActions
  (params (AgentIds :type Array%20of%20Integers))
  (for _array_element AgentIds
    (Utilities|FlowControl|Sequence
      (:then_0
        (bind _returnvalue (Class|FloatAction|GetFloatAction (Variables|Default|GetThrottleBrakeAction) _array_element))
        (if (> _returnvalue 0.0)
          (Variables|/Game/FlyingGame/Blueprints/BP_BestPlane.BP_BestPlane_C|SetThrottleAmount (Class|LearningAgentsManagerComponent|GetAgent _array_element "/Game/FlyingGame/Blueprints/BP_BestPlane.BP_BestPlane_C") (Math|Float|Truncate (* _returnvalue 1e+02)))))
      (:then_1
        (bind _returnvalue_2 (Class|FloatAction|GetFloatAction (Variables|Default|GetLeft%20Right%20Movement) _array_element))
        (Class|PrimitiveComponent|AddTorqueinDegrees (Variables|/Game/FlyingGame/Blueprints/BP_BestPlane.BP_BestPlane_C|GetDriver (Class|LearningAgentsManagerComponent|GetAgent _array_element "/Game/FlyingGame/Blueprints/BP_BestPlane.BP_BestPlane_C")) (Math|Vector|Lerp(Vector) "0, 0, 0" (* (Math|Vector|GetUpVector (Variables|/Game/FlyingGame/Blueprints/BP_BestPlane.BP_BestPlane_C|GetDriver (Class|LearningAgentsManagerComponent|GetAgent _array_element "/Game/FlyingGame/Blueprints/BP_BestPlane.BP_BestPlane_C"))) (* (* _returnvalue_2 7.5) (Variables|Default|GetAircontrol))) 0.1) "None" true))
      (:then_2
        (bind _returnvalue_3 (Class|FloatAction|GetFloatAction (Variables|Default|GetUp%20Down%20Movement) _array_element))
        (Class|PrimitiveComponent|AddTorqueinDegrees (Variables|/Game/FlyingGame/Blueprints/BP_BestPlane.BP_BestPlane_C|GetDriver (Class|LearningAgentsManagerComponent|GetAgent _array_element "/Game/FlyingGame/Blueprints/BP_BestPlane.BP_BestPlane_C")) (Math|Vector|Lerp(Vector) "0, 0, 0" (* (Math|Vector|GetRightVector (Variables|/Game/FlyingGame/Blueprints/BP_BestPlane.BP_BestPlane_C|GetDriver (Class|LearningAgentsManagerComponent|GetAgent _array_element "/Game/FlyingGame/Blueprints/BP_BestPlane.BP_BestPlane_C"))) (* _returnvalue_3 (Variables|Default|GetAircontrol))) 0.1) "None" true))
      (:then_3
        (bind _returnvalue_4 (Class|FloatAction|GetFloatAction (Variables|Default|GetRoll%20Movement) _array_element))
        (Class|PrimitiveComponent|AddTorqueinDegrees (Variables|/Game/FlyingGame/Blueprints/BP_BestPlane.BP_BestPlane_C|GetDriver (Class|LearningAgentsManagerComponent|GetAgent _array_element "/Game/FlyingGame/Blueprints/BP_BestPlane.BP_BestPlane_C")) (Math|Vector|Lerp(Vector) "0, 0, 0" (* (Math|Vector|GetForwardVector (Variables|/Game/FlyingGame/Blueprints/BP_BestPlane.BP_BestPlane_C|GetDriver (Class|LearningAgentsManagerComponent|GetAgent _array_element "/Game/FlyingGame/Blueprints/BP_BestPlane.BP_BestPlane_C"))) (* _returnvalue_4 (Variables|Default|GetAircontrol))) 0.1) "None" true)))))